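; Sowing placement indicator actor that previews where a growable would go and whether that spot is taken.
; Update moves it, syncs mesh and blocking radius from the CoreManager subsystem, and drives the dynamic material: strobing when clear, occupancy-scaled brightness when blocked.
; Each tick, sphere overlaps with kernels, organic growables or static-mesh actors set the subsystem's already-occupied flag.
; The sphere's visibility follows a debugger command.
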(event Custom|Update
  (params (Center :type Vector) (Normal :type Vector) (State :type EWidgetState%20Enum :default "kClear") (Occupied :type Float%20%28double-precision%29))
  (bind _ring_dynamic_material_instance (Variables|Default|GetRing%20Dynamic%20Material%20Instance))
  (Transformation|SetActorLocationAndRotation Center "0, 0, 0")
  (CallFunction|AdjustStaticMesh)
  (CallFunction|AdjustSphereRadius)
  (switch Utilities|FlowControl|Switch|SwitchonEWidgetState State
    (:kClear
      (Rendering|Material|SetScalarParameterValue _ring_dynamic_material_instance "Brightness" (Variables|Default|GetBrightnessClear) :!class /Script/Engine.MaterialInstanceDynamic)
      (Rendering|Material|SetScalarParameterValue (Variables|Default|GetRing%20Dynamic%20Material%20Instance) "StrobeRate" 2.0 :!class /Script/Engine.MaterialInstanceDynamic))
    (:kBlocked
      (Rendering|Material|SetScalarParameterValue _ring_dynamic_material_instance "Brightness" (Math|Float|Lerp 0.0 15.0 (Math|Float|Square Occupied)) :!class /Script/Engine.MaterialInstanceDynamic)
      (Rendering|Material|SetScalarParameterValue (Variables|Default|GetRing%20Dynamic%20Material%20Instance) "StrobeRate" 0.0 :!class /Script/Engine.MaterialInstanceDynamic))))

(event EventBeginPlay
  (bind _returnvalue (Rendering|Material|CreateDynamicMaterialInstance (Variables|Default|GetSM_Ring) 0 0 "None" :!class /Script/Engine.PrimitiveComponent))
  (Variables|Default|SetRing%20Dynamic%20Material%20Instance _returnvalue))

(event EventTick
  (params (DeltaSeconds :type Float%20%28single-precision%29))
  (CallFunction|CheckOverlapping)
  (if (not (Variables|Rendering|GetbHidden))
    (Development|SetHiddeninGame (Variables|Default|GetSphere) (not (Class|HelperBlueprintFunction|IsDebuggerCommandActive)) false)))

(fn ConstructionScript)

(fn GetBrightness
  (params (State :type EWidgetState%20Enum :default "kClear") (OccupiedPercentage :type Float%20%28double-precision%29)))

(fn AdjustStaticMesh
  (bind _returnvalue (Subsystems|GetCoreManagerSubSystem))
  (bind _sm_ring (Variables|Default|GetSM_Ring))
  (bind _returnvalue_2 (Class|CoreManagerSubSystem|GetGrowableStaticMesh _returnvalue))
  (Components|StaticMesh|SetStaticMesh _sm_ring (select (Utilities|IsValid _returnvalue_2) _returnvalue_2 (Variables|Default|GetRing)))
  (for (_ _array_index) (Rendering|Material|GetMaterials _sm_ring)
    (Rendering|Material|SetMaterial _sm_ring _array_index (Variables|Default|GetRing%20Dynamic%20Material%20Instance))))

(fn AdjustSphereRadius
  (bind _returnvalue (Subsystems|GetCoreManagerSubSystem))
  (bind _sphere (Variables|Default|GetSphere))
  (bind _returnvalue_2 (Class|CoreManagerSubSystem|GetGrowableBlockingRadius _returnvalue))
  (if (not (== (Components|Sphere|GetScaledSphereRadius _sphere) _returnvalue_2))
    (Components|Sphere|SetSphereRadius _sphere _returnvalue_2 true)))

(fn CheckOverlapping
  (LocalVariables|SetIsOverlapping false)
  (bind _array_element (Utilities|Array|ForEachLoopwithBreak (Collision|GetOverlappingActors (Variables|Default|GetSphere) "/Script/Engine.Actor" :!class /Script/Engine.PrimitiveComponent) :!label _label)
    (:LoopBody
      (Utilities|Casting|CastToBP_Kernel _array_element
        (:then
          _)
        (:CastFailed
          (Utilities|Casting|CastToBP_Growable_Organic _array_element
            (:then
              _)
            (:CastFailed
              (Utilities|IsValid (Actor|GetComponentbyClass _array_element "/Script/Engine.StaticMeshComponent")
                (:Is%20Valid
                  _))))))
      (LocalVariables|SetIsOverlapping true)
      (goto _label Break))
    (:Completed
      (Class|CoreManagerSubSystem|SetSowingAlreadyOccupied (Subsystems|GetCoreManagerSubSystem) (LocalVariables|GetIsOverlapping)))))