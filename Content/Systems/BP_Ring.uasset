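; BP_Ring is a one-shot decal ring effect that starts on BeginPlay and destroys itself when finished.
; BeginPlay creates a dynamic instance of the decal material, without assigning it back to the decal, and caches its base Glowiness.
; A timeline, rate-scaled by Duration, drives actor scale toward TargetScale and sets the instance's Opacity and Glowiness from an intensity curve.
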(event Custom|Trigger
  (bind _glowmaterial (Variables|Default|GetGlowMaterial))
  (Components|Timeline|SetPlayRate (Variables|Default|GetTimeline) (/ 1.0 (Variables|Default|GetDuration)))
  (bind (_direction _scale _intensity) (Timeline|Timeline Play)
    (:Update
      (Transformation|SetActorScale3D (Math|Conversions|ToVector(Float) (* _scale (Variables|Default|GetTargetScale))))
      (Rendering|Material|SetScalarParameterValue _glowmaterial "Opacity" _intensity :!class /Script/Engine.MaterialInstanceDynamic)
      (Rendering|Material|SetScalarParameterValue _glowmaterial "Glowiness" (* _intensity (Variables|Default|GetGlowiness)) :!class /Script/Engine.MaterialInstanceDynamic))
    (:Finished
      (Actor|DestroyActor))))

(event EventBeginPlay
  (bind _returnvalue (Rendering|Material|CreateDynamicMaterialInstance (Class|DecalComponent|GetDecalMaterial (Variables|Default|GetDecal)) "None" "None" :!class /Script/Engine.KismetMaterialLibrary))
  (bind _output_get (Variables|Default|SetGlowMaterial _returnvalue))
  (bind _returnvalue_2 (Rendering|Material|GetScalarParameterValue _output_get "Glowiness" :!class /Script/Engine.MaterialInstanceDynamic))
  (Variables|Default|SetGlowiness _returnvalue_2)
  (CallFunction|Trigger))

(event Collision|EventActorBeginOverlap
  (params (OtherActor :type Actor%20Object%20Reference)))

(event EventTick
  (params (DeltaSeconds :type Float%20%28single-precision%29)))

(fn ConstructionScript)