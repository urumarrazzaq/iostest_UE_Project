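; BP_Orbiter is an actor that circles the world origin around the Y axis at radius Distance, with its Arrow pointing at the center.
; Tick grows Angle by DeltaSeconds, rotates an X offset by a quaternion and sets the result as world location.
; A look-at rotation from that point to zero aims the Arrow.
; QuatFromAxisAngle builds the quaternion by hand using the half-angle sine and cosine formula.
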(event EventBeginPlay)

(event Collision|EventActorBeginOverlap
  (params (OtherActor :type Actor%20Object%20Reference)))

(event EventTick
  (params (DeltaSeconds :type Float%20%28single-precision%29))
  (bind _output_get (Variables|Default|SetAngle (+ DeltaSeconds (Variables|Default|GetAngle))))
  (bind _outquat (CallFunction|QuatfromAxisAngle _output_get (Math|Vector|MakeVector 0.0 1.0 0.0)))
  (Transformation|SetActorLocation (Class|KismetMathLibrary|QuatRotateVector _outquat (Math|Vector|MakeVector (Variables|Default|GetDistance) 0.0 0.0)) false false)
  (Transformation|SetWorldRotation (Variables|Default|GetArrow) (Math|Rotator|FindLookatRotation (Class|KismetMathLibrary|QuatRotateVector _outquat (Math|Vector|MakeVector (Variables|Default|GetDistance) 0.0 0.0)) (Math|Vector|VectorZero)) false false))

(fn ConstructionScript)

(fn QuatfromAxisAngle
  (params (Angle :type Float%20%28double-precision%29) (Axis :type Vector))
  (bind _returnvalue (/ Angle 2.0))
  (bind _returnvalue_2 (Math|Trig|Sin(Radians) _returnvalue))
  (bind _returnvalue_3 (* Axis _returnvalue_2))
  (return (Class|KismetMathLibrary|MakeQuat (.x _returnvalue_3) (.y _returnvalue_3) (.z _returnvalue_3) (Math|Trig|Cos(Radians) _returnvalue))))