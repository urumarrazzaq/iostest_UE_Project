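; Light manager for the stylized grass environment that switches the scene between day and night presets.
; NightToDay and DayToNight set Sun and Moon intensity, the active light's rotation and colour, skylight, and height fog, then update IsDay.
; Both also push wind colour and strength into the MPC_WindStrength material parameter collection.
; The construction script and BeginPlay apply the preset chosen by IsDay, instantly and without blending.
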(event EventBeginPlay
  (if (Variables|Controls|GetbIsDay?)
    (CallFunction|NighttoDay)
    (else
      (CallFunction|DaytoNight))))

(fn ConstructionScript
  (if (Variables|Controls|GetbIsDay?)
    (CallFunction|NighttoDay)
    (else
      (CallFunction|DaytoNight))))

(fn UpdateWindColour
  (params (WindColourAmount :type Float%20%28double-precision%29))
  (Rendering|Material|SetScalarParameterValue "/Game/StylizedGrass/MaterialParameterCollections/MPC_WindStrength.MPC_WindStrength" "WindColourIntensity" WindColourAmount :!class /Script/Engine.KismetMaterialLibrary))

(fn DaytoNight
  (Utilities|FlowControl|Sequence
    (:then_0
      (Rendering|Components|Light|SetIntensity (Variables|/Script/Engine.Light|GetLightComponent (Variables|References|GetSun)) (Variables|Sun|GetSunIntensity_Night)))
    (:then_1
      (Transformation|SetActorRotation (Variables|References|GetMoon) (Variables|Moon|GetMoonPosition_Night)))
    (:then_2
      (Class|ExponentialHeightFogComponent|SetDirectionalInscatteringColor (Variables|/Script/Engine.ExponentialHeightFog|GetComponent (Variables|References|GetExponentialHeightFog)) (Variables|Fog|GetDirectionalInscatteringColour_Night)))
    (:then_3
      (Class|ExponentialHeightFogComponent|SetVolumetricFogEmissive (Variables|/Script/Engine.ExponentialHeightFog|GetComponent (Variables|References|GetExponentialHeightFog)) (Variables|Fog|GetVF_Emissive_Night)))
    (:then_4
      (Class|SkyLightComponent|SetOcclusionTint (Variables|/Script/Engine.SkyLight|GetLightComponent (Variables|References|GetSkylight)) (Variables|Skylight|GetOcclusion_Tint_Night)))
    (:then_5
      (Rendering|Components|Light|SetIntensity (Variables|/Script/Engine.SkyLight|GetLightComponent (Variables|References|GetSkylight)) (Variables|Skylight|GetSkylight_Intensity_Night)))
    (:then_6
      (Rendering|Components|Light|SetLightColor (Variables|/Script/Engine.Light|GetLightComponent (Variables|References|GetMoon)) (Variables|Moon|GetMoonColour_Night) true))
    (:then_7
      (Class|ExponentialHeightFogComponent|SetVolumetricFogAlbedo (Variables|/Script/Engine.ExponentialHeightFog|GetComponent (Variables|References|GetExponentialHeightFog)) (Variables|Fog|GetVF_Albedo_Night)))
    (:then_8
      (Class|ExponentialHeightFogComponent|SetFogInscatteringColor (Variables|/Script/Engine.ExponentialHeightFog|GetComponent (Variables|References|GetExponentialHeightFog)) (Variables|Fog|GetFogInscatteringColour_Night)))
    (:then_9
      (Class|ExponentialHeightFogComponent|SetFogDensity (Variables|/Script/Engine.ExponentialHeightFog|GetComponent (Variables|References|GetExponentialHeightFog)) (Variables|Fog|GetFog_Density_Night)))
    (:then_10
      (CallFunction|UpdateWindColour (Variables|Wind|GetWindColourAmount_Night)))
    (:then_11
      (Rendering|Components|Light|SetIntensity (Variables|/Script/Engine.Light|GetLightComponent (Variables|References|GetMoon)) (Variables|Moon|GetMoonIntensity_Night)))
    (:then_12
      (CallFunction|UpdateWindAmount (Variables|Wind|GetWind%20Amount)))
    (:then_13
      (Variables|Controls|SetbIsDay? false))))

(fn NighttoDay
  (Utilities|FlowControl|Sequence
    (:then_0
      (Rendering|Components|Light|SetIntensity (Variables|/Script/Engine.Light|GetLightComponent (Variables|References|GetSun)) (Variables|Sun|GetSunIntensity_Day)))
    (:then_1
      (Transformation|SetActorRotation (Variables|References|GetSun) (Variables|Sun|GetSunPosition_Day)))
    (:then_2
      (Class|ExponentialHeightFogComponent|SetDirectionalInscatteringColor (Variables|/Script/Engine.ExponentialHeightFog|GetComponent (Variables|References|GetExponentialHeightFog)) (Variables|Fog|GetDirectionalInscatteringColour_Day)))
    (:then_3
      (Class|ExponentialHeightFogComponent|SetVolumetricFogEmissive (Variables|/Script/Engine.ExponentialHeightFog|GetComponent (Variables|References|GetExponentialHeightFog)) (Variables|Fog|GetVF_Emissive_Day)))
    (:then_4
      (Class|SkyLightComponent|SetOcclusionTint (Variables|/Script/Engine.SkyLight|GetLightComponent (Variables|References|GetSkylight)) (Variables|Skylight|GetOcclusion_Tint_Day)))
    (:then_5
      (Rendering|Components|Light|SetIntensity (Variables|/Script/Engine.SkyLight|GetLightComponent (Variables|References|GetSkylight)) (Variables|Skylight|GetSkylight_Intensity_Day)))
    (:then_6
      (Rendering|Components|Light|SetLightColor (Variables|/Script/Engine.Light|GetLightComponent (Variables|References|GetSun)) (Variables|Sun|GetLightColour_Day) true))
    (:then_7
      (Class|ExponentialHeightFogComponent|SetVolumetricFogAlbedo (Variables|/Script/Engine.ExponentialHeightFog|GetComponent (Variables|References|GetExponentialHeightFog)) (Variables|Fog|GetVF_Albedo_Day)))
    (:then_8
      (Class|ExponentialHeightFogComponent|SetFogInscatteringColor (Variables|/Script/Engine.ExponentialHeightFog|GetComponent (Variables|References|GetExponentialHeightFog)) (Variables|Fog|GetFogInscatteringColour_Day)))
    (:then_9
      (Class|ExponentialHeightFogComponent|SetFogDensity (Variables|/Script/Engine.ExponentialHeightFog|GetComponent (Variables|References|GetExponentialHeightFog)) (Variables|Fog|GetFog_Density_Day)))
    (:then_10
      (CallFunction|UpdateWindColour (Variables|Wind|GetWindColourAmount_Day)))
    (:then_11
      (Rendering|Components|Light|SetIntensity (Variables|/Script/Engine.Light|GetLightComponent (Variables|References|GetMoon)) (Variables|Moon|GetMoonIntensity_Day)))
    (:then_12
      (CallFunction|UpdateWindAmount (Variables|Wind|GetWind%20Amount)))
    (:then_13
      (Variables|Controls|SetbIsDay? true))))

(fn UpdateWindAmount
  (params (WindAmount :type Float%20%28double-precision%29))
  (Rendering|Material|SetScalarParameterValue "/Game/StylizedGrass/MaterialParameterCollections/MPC_WindStrength.MPC_WindStrength" "WindIntensity" WindAmount :!class /Script/Engine.KismetMaterialLibrary))