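; BP_GrowableFlowers01_Illustrated is a flower actor, named as a growable variant, that gets a randomly tinted material at runtime.
; On BeginPlay it runs the parent logic, then creates a dynamic material instance from the mesh's first material slot.
; It sets a fixed wildflower texture and a random Color from ColorPallete, then applies the instance to the mesh.
; An author note flags that the texture should match this actor's mesh.
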(event EventBeginPlay
  (|CallParentFunction)
  (CallFunction|SetDynamicMaterial))

(fn ConstructionScript
  (|CallParentFunction))

(fn SetDynamicMaterial
  (bind _returnvalue (Rendering|Material|CreateDynamicMaterialInstance (Variables|Character|GetMesh) 0 (Rendering|Material|GetMaterial (Variables|Character|GetMesh) 0) "None" :!class /Script/Engine.PrimitiveComponent))
  (LocalVariables|SetMaterial _returnvalue)
  ;[0.5906 0.4999 0 0.5] This should be updated so that the Value parameter corresponds to the correct texture for this actor's mesh
  (Rendering|Material|SetTextureParameterValue (LocalVariables|GetMaterial) "Texture" "/Game/Art/SmallPlants/t_stylizedwildflowers_d_720.t_stylizedwildflowers_d_720")
  (Rendering|Material|SetVectorParameterValue (LocalVariables|GetMaterial) "Color" (.OutItem (Utilities|Array|Random (Variables|Default|GetColorPallete))) :!class /Script/Engine.MaterialInstanceDynamic)
  (Rendering|Material|SetMaterial (Variables|Character|GetMesh) 0 (LocalVariables|GetMaterial)))