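; Actor component that changes the landscape's look as growables are added or removed, shifting between sand and grass.
; Per-HealthType enhance values from the core config are added to or subtracted from running totals, written to a Material Parameter Collection.
; Additions enable a temporary Tick blend unless skipped.
; The SandToGrass parameter also drives falling-leaves Niagara rate and color, post-process gamma and saturation, and threshold-based butterfly spawning.
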(event Custom|OnAddingGrowables
  (params (SkipProcessingTime :type Boolean) (TimeInterval :type Float%20%28double-precision%29) (healthType :type EHealthDataType%20Enum :default "MoveCalories"))
  (Variables|Default|SetSkipGrowingProcess SkipProcessingTime)
  (Variables|Default|SetTime%20Interval TimeInterval)
  (CallFunction|FinalizeCurrentMaterialParameter)
  (CallFunction|AddNumberOfGrowables healthType)
  (if (not (Variables|Default|GetSkipGrowingProcess))
    (Variables|Default|SetAlpha 0.0)
    (Components|Tick|SetComponentTickEnabled true)))

(event Custom|OnGrowableDestroied
  (params (HealthType :type EHealthDataType%20Enum :default "MoveCalories"))
  (CallFunction|RemovefromNumberOfGrowables HealthType)
  (CallFunction|FinalizeCurrentMaterialParameter))

(event Custom|FinalizeCurrentMaterialParameter
  (bind _currentmaterialparametervalue (Variables|Default|GetCurrentMaterialParameterValue))
  (Variables|Default|SetTotalMaterialParameterValue (Variables|Default|GetCurrentMaterialParameterValue))
  (for _array_element (.materialparameters _currentmaterialparametervalue)
    (Rendering|Material|SetScalarParameterValue (.materialparametercollection _currentmaterialparametervalue) (.materialparametername _array_element) (.parameterenhancevalue _array_element) :!class /Script/Engine.KismetMaterialLibrary)
    (CallFunction|UpdateFallingLeavesSystem)
    (CallFunction|SpawnorDespawnButterflies)
    (CallFunction|UpdatePostProcessSaturation)))

(event Custom|ResetMaterialParameters
  (params (NewDate :type Date%20Time%20Structure))
  ;[0.15 0.15 0.15 0.5] This is a sloppy mess for now- attempting to fix landscape material parameters not updating when day is changed -ND
)

(event Custom|Test
  ;[0.15 0.15 0.15 0.5] This is a sloppy mess for now- attempting to fix landscape material parameters not updating when day is changed -ND
  (Utilities|FlowControl|Delay 0.2)
  (Development|PrintString "Reset")
  (CallFunction|ResetGrowablesandVisual))

(event EventBeginPlay
  (bind _returnvalue (Actor|GetActorOfClass "/Script/Engine.PostProcessVolume"))
  (Variables|Default|SetPostProcessVolume _returnvalue)
  (CallFunction|InitializeFallingLeavesSystem)
  (CallFunction|FinalizeCurrentMaterialParameter)
  (Components|Tick|SetComponentTickEnabled false)
  (EventDispatchers|BindEventtoOnGrowableAdded (EventDispatchers|CreateEvent :!event Custom|OnAddingGrowables))
  (EventDispatchers|BindEventtoOnGrowableRemoved (EventDispatchers|CreateEvent :!event Custom|OnGrowableDestroied))
  ;[0.107 0.08228 0.2307] Untill we figure out better way to handle it
  ; For loading a saved game
  (Utilities|FlowControl|Delay 0.1)
  (Default|CallOnLandscapeFinalized)
  (if (Variables|Default|GetSkipGrowingProcess)
    (CallFunction|FinalizeCurrentMaterialParameter)))

(event EventEndPlay
  (params (EndPlayReason :type EEndPlayReason%20Enum :default "Destroyed"))
  (EventDispatchers|UnbindallEventsfromOnGrowableAdded))

(event EventTick
  (params (DeltaSeconds :type Float%20%28single-precision%29))
  (bind _currentmaterialparametervalue (Variables|Default|GetCurrentMaterialParameterValue))
  ;[0.107 0.08228 0.2307] Change of the landscape material
  (bind _output_get (Variables|Default|SetAlpha (Math|Float|Clamp(Float) (Math|Interpolation|FInterptoConstant (Variables|Default|GetAlpha) 1.0 DeltaSeconds (Variables|Default|GetTime%20Interval)))))
  (if (Math|Float|NearlyEqual(Float) _output_get 1.0 1e-06)
    (Components|Tick|SetComponentTickEnabled false)
    (CallFunction|FinalizeCurrentMaterialParameter)
    (else
      (CallFunction|UpdatePostProcessSaturation)
      (for (_array_element _array_index) (.materialparameters _currentmaterialparametervalue)
        (Rendering|Material|SetScalarParameterValue (.materialparametercollection _currentmaterialparametervalue) (.materialparametername _array_element) (Math|Float|Clamp(Float) (Math|Float|Lerp (.parameterenhancevalue _array_element) (.parameterenhancevalue (Utilities|Array|Get(acopy) (.materialparameters (Variables|Default|GetTotalMaterialParameterValue)) _array_index)) (Variables|Default|GetAlpha))) :!class /Script/Engine.KismetMaterialLibrary)))))

(fn AddNumberOfGrowables
  (params (HealthType :type EHealthDataType%20Enum :default "MoveCalories"))
  (bind _returnvalue (Subsystems|GetCoreManagerSubSystem))
  (bind _currentmaterialparametervalue (Variables|Default|GetCurrentMaterialParameterValue))
  (bind _coreconfig (Variables|/Script/iostest.CoreManagerSubSystem|GetCoreConfig _returnvalue))
  (Utilities|IsValid _coreconfig
    (:Is%20Valid
      (LocalVariables|SetlocalCoreConfig _coreconfig)
      (if (.ReturnValue (Utilities|Map|Find (Variables|Default|GetNumberOfGrowables) HealthType))
        (for _array_element (.materialparameters (.Value (Utilities|Map|Find (Class|CoreConfig|GetLandscapeEnhanceValues (LocalVariables|GetlocalCoreConfig)) HealthType)))
          (Utilities|Array|Add (LocalVariables|GetlocalMaterial) _array_element))
        (for _array_element_2 (LocalVariables|GetlocalMaterial)
          (for (_array_element_3 _array_index) (.materialparameters _currentmaterialparametervalue)
            (if (== (.materialparametername _array_element_3) (.materialparametername _array_element_2))
              (Utilities|Array|SetArrayElem (.materialparameters _currentmaterialparametervalue) _array_index (Utilities|Struct|MakeLandscapeConfig (.materialparametername _array_element_3) (+ (.parameterenhancevalue _array_element_3) (.parameterenhancevalue _array_element_2)))))))))
    (:Is%20Not%20Valid
      (Development|PrintString "No Valid Core Config"))))

(fn UpdateFallingLeavesSystem
  (Utilities|IsValid (Variables|Default|GetFallingLeavesSystem)
    (:Is%20Valid
      (bind _returnvalue (Rendering|Material|GetScalarParameterValue (.materialparametercollection (Variables|Default|GetTotalMaterialParameterValue)) (Utilities|Name|MakeLiteralName "SandToGrass") :!class /Script/Engine.KismetMaterialLibrary))
      (LocalVariables|SetAlpha _returnvalue)
      (Niagara|SetNiagaraVariable(Float) (Variables|Default|GetFallingLeavesSystem) "SpawnRate" (Math|Float|MapRangeClamped (LocalVariables|GetAlpha) 0.0 0.6 (LocalVariables|GetSpawnRateMin) (LocalVariables|GetSpawnRateMax)))
      (Niagara|SetNiagaraVariable(Float) (Variables|Default|GetFallingLeavesSystem) "LeafColorMin" (Math|Float|MapRangeClamped (LocalVariables|GetAlpha) 0.0 0.6 0.5 0.0))
      (Niagara|SetNiagaraVariable(Float) (Variables|Default|GetFallingLeavesSystem) "LeafColorMax" (Math|Float|MapRangeClamped (LocalVariables|GetAlpha) 0.0 0.6 1.0 0.5))
      (if false ; DEBUG: Show all Debug Text
        (Development|PrintString (Utilities|String|Append "Alpha: " (Utilities|String|ToString(Float) (LocalVariables|GetAlpha)) "| LeafColorMin: " (Utilities|String|ToString(Float) (Math|Float|MapRangeClamped (LocalVariables|GetAlpha) 0.0 0.6 0.5 0.0)) "| LeafColorMax: " (Utilities|String|ToString(Float) (Math|Float|MapRangeClamped (LocalVariables|GetAlpha) 0.0 0.6 1.0 0.5)) "SpawnRate: " (Utilities|String|ToString(Float) (Math|Float|MapRangeClamped (LocalVariables|GetAlpha) 0.0 0.6 (LocalVariables|GetSpawnRateMin) (LocalVariables|GetSpawnRateMax)))) true true "(R=0.000000,G=0.660000,B=1.000000,A=1.000000)" 3e+01 "FallingLeavesDebugStrings")))))

(fn InitializeFallingLeavesSystem
  ;[0.15 0.15 0.15 0.5] Set reference variable FallingLeavesSytstem by searching the level for the Niagara Actor of the correct type
  (bind _outactors (Actor|GetAllActorsOfClass "/Script/Niagara.NiagaraActor"))
  (for _array_element _outactors
    (if (== (AssetData|GetAsset (Variables|/Script/Niagara.NiagaraActor|GetNiagaraComponent _array_element)) "/Game/VFX/WindblownParticles/NS_FallingLeaves.NS_FallingLeaves")
      (Variables|Default|SetFallingLeavesSystem (Variables|/Script/Niagara.NiagaraActor|GetNiagaraComponent _array_element)))))

(fn ResetGrowablesandVisual
  (Utilities|Map|Clear (Variables|Default|GetNumberOfGrowables))
  (Variables|Default|SetCurrentMaterialParameterValue (Variables|Default|GetEmptyMaterialParameterValue))
  (CallFunction|FinalizeCurrentMaterialParameter))

(fn SpawnorDespawnButterflies
  ;[0.15 0.15 0.15 0.5] Update Alpha Value
  (bind _returnvalue (Rendering|Material|GetScalarParameterValue (.materialparametercollection (Variables|Default|GetTotalMaterialParameterValue)) (Utilities|Name|MakeLiteralName "SandToGrass") :!class /Script/Engine.KismetMaterialLibrary))
  (LocalVariables|SetAlpha _returnvalue)
  (bind _keys (Utilities|Map|Keys (Variables|Default|GetButterflySpawnThresholds)))
  (for _array_element _keys
    (if (>= (LocalVariables|GetAlpha) _array_element)
      ;[0.15 0.15 0.15 0.5] If the current Alpha value is greater than the threshold currently being testeed, spawn butterflies X times where X is the amount designated by the threshold currently being tested minus the number of butterflies already in the level
      (if (< (Utilities|Array|Length (Variables|Default|GetButterfliesSpawned)) (.Value (Utilities|Map|Find (Variables|Default|GetButterflySpawnThresholds) _array_element)))
        (for _index (range 1 (- (.Value (Utilities|Map|Find (Variables|Default|GetButterflySpawnThresholds) _array_element)) (Utilities|Array|Length (Variables|Default|GetButterfliesSpawned))))
          (bind _returnvalue_2 (Game|SpawnActorfromClass "/Game/Blueprints/Butterfly/BP_Butterfly.BP_Butterfly_C" (Math|Transform|MakeTransform "0, 0, 0" (Math|Random|RandomRotator true) "1.000000,1.000000,1.000000") "AdjustIfPossibleButAlwaysSpawn" "MultiplyWithRoot" 0 0))
          (Utilities|Array|Add (Variables|Default|GetButterfliesSpawned) _returnvalue_2)
          ;[0.15 0.15 0.15 0.5] Teleport spawned butterfly to random spots within landscape bounding box (raised and slightly shrunk) until not overlapping anything
          (Utilities|FlowControl|ForLoopwithBreak 0 500 :!label _label
            (:LoopBody
              (bind _returnvalue_3 (Actor|GetActorOfClass "/Script/Landscape.Landscape"))
              (Transformation|SetActorLocation _returnvalue_2 (Math|Random|RandomPointinBoundingBox (+ (.Origin (Collision|GetComponentBounds (Actor|GetComponentbyClass _returnvalue_3 "/Script/Landscape.LandscapeComponent"))) "0.000000,0.000000,300.000000") (* (.BoxExtent (Collision|GetComponentBounds (Actor|GetComponentbyClass _returnvalue_3 "/Script/Landscape.LandscapeComponent"))) 0.8)) false false)
              ;[0.15 0.15 0.15 0.5] Line trace straight up to make sure we're not trapped inside some geometry
              (bind _returnvalue_4 (Collision|LineTraceForObjects (Transformation|GetActorLocation _returnvalue_2) (+ (Transformation|GetActorLocation _returnvalue_2) (* (Math|Vector|VectorUp) 1e+04)) (Utilities|Array|MakeArray "ObjectTypeQuery1") true 0 "None"))
              (if (and (Utilities|Array|IsEmpty (Collision|GetOverlappingActors _returnvalue_2 "/Script/Engine.Actor" :!class /Script/Engine.Actor)) (not _returnvalue_4))
                (goto _label Break))))))
      (else
        ;[0.15 0.15 0.15 0.5] If the current Alpha value is less than the threshold currently being tested, remove X butterflies from the level where X is the number of butterflies in the level minus the number of butterflies designated by the threshold
        (if (not (< (Utilities|Array|Length (Variables|Default|GetButterfliesSpawned)) (.Value (Utilities|Map|Find (Variables|Default|GetButterflySpawnThresholds) _array_element))))
          (Utilities|Array|Shuffle (Variables|Default|GetButterfliesSpawned))
          (for _index_2 (range 0 (- (Utilities|Array|Length (Variables|Default|GetButterfliesSpawned)) (.Value (Utilities|Map|Find (Variables|Default|GetButterflySpawnThresholds) _array_element))))
            (Actor|DestroyActor (Utilities|Array|Get(acopy) (Variables|Default|GetButterfliesSpawned) _index_2))
            (Utilities|Array|RemoveIndex (Variables|Default|GetButterfliesSpawned) _index_2)))))))

(fn UpdatePostProcessSaturation
  (bind _returnvalue (Rendering|Material|GetScalarParameterValue (.materialparametercollection (Variables|Default|GetTotalMaterialParameterValue)) (Utilities|Name|MakeLiteralName "SandToGrass") :!class /Script/Engine.KismetMaterialLibrary))
  (Utilities|Struct|SetmembersinPostProcessSettings (Variables|/Script/Engine.PostProcessVolume|GetSettings (Variables|Default|GetPostProcessVolume)) (Math|Vector4|MakeVector4 (Math|Float|MapRangeClamped _returnvalue 0.0 0.5 0.9 1.0) (Math|Float|MapRangeClamped _returnvalue 0.0 0.5 0.9 1.0) (Math|Float|MapRangeClamped _returnvalue 0.0 0.5 0.9 1.0) (Math|Float|MapRangeClamped _returnvalue 0.0 0.5 0.9 1.0)) (Math|Vector4|MakeVector4 (Math|Float|MapRangeClamped _returnvalue 0.0 0.5 0.75 1.05) (Math|Float|MapRangeClamped _returnvalue 0.0 0.5 0.75 1.05) (Math|Float|MapRangeClamped _returnvalue 0.0 0.5 0.75 1.05) (Math|Float|MapRangeClamped _returnvalue 0.0 0.5 0.75 1.05)) (Math|Vector4|MakeVector4 (Math|Float|MapRangeClamped _returnvalue 0.0 0.5 0.75 1.05) (Math|Float|MapRangeClamped _returnvalue 0.0 0.5 0.75 1.05) (Math|Float|MapRangeClamped _returnvalue 0.0 0.5 0.75 1.05) (Math|Float|MapRangeClamped _returnvalue 0.0 0.5 0.75 1.05)) (Math|Vector4|MakeVector4 (Math|Float|MapRangeClamped _returnvalue 0.0 0.5 0.75 1.05) (Math|Float|MapRangeClamped _returnvalue 0.0 0.5 0.75 1.05) (Math|Float|MapRangeClamped _returnvalue 0.0 0.5 0.75 1.05) (Math|Float|MapRangeClamped _returnvalue 0.0 0.5 0.75 1.05))))

(fn RemovefromNumberOfGrowables
  (params (HealthType :type EHealthDataType%20Enum :default "MoveCalories"))
  (bind _returnvalue (Subsystems|GetCoreManagerSubSystem))
  (bind _currentmaterialparametervalue (Variables|Default|GetCurrentMaterialParameterValue))
  (bind _coreconfig (Variables|/Script/iostest.CoreManagerSubSystem|GetCoreConfig _returnvalue))
  (Utilities|IsValid _coreconfig
    (:Is%20Valid
      (LocalVariables|SetlocalCoreConfig _coreconfig)
      (if (.ReturnValue (Utilities|Map|Find (Variables|Default|GetNumberOfGrowables) HealthType))
        (for _array_element (.materialparameters (.Value (Utilities|Map|Find (Class|CoreConfig|GetLandscapeEnhanceValues (LocalVariables|GetlocalCoreConfig)) HealthType)))
          (Utilities|Array|Add (LocalVariables|GetlocalMaterial) _array_element))
        (for _array_element_2 (LocalVariables|GetlocalMaterial)
          (for (_array_element_3 _array_index) (.materialparameters _currentmaterialparametervalue)
            (if (== (.materialparametername _array_element_3) (.materialparametername _array_element_2))
              (Utilities|Array|SetArrayElem (.materialparameters _currentmaterialparametervalue) _array_index (Utilities|Struct|MakeLandscapeConfig (.materialparametername _array_element_3) (- (.parameterenhancevalue _array_element_3) (.parameterenhancevalue _array_element_2)))))))))
    (:Is%20Not%20Valid
      (Development|PrintString "No Valid Core Config"))))