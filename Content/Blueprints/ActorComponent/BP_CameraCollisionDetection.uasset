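; Actor component that checks whether a zoom, rotation or pan of the owning Maru character's camera would hit an obstacle.
; It caches the owner's CameraComponent on BeginPlay, then offers three queries that trace ahead on the Camera channel and return the hit result.
; Zoom and pan sweep spheres along the movement, while rotation casts a line along camera up/right vectors weighted by quaternion components, flipping vertical sign with yaw.
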(event EventBeginPlay
  (bind _output_get (Variables|Default|SetMaruCharacter (Components|GetOwner)))
  (Variables|Default|SetMaruCamera (Actor|GetComponentbyClass _output_get "/Script/Engine.CameraComponent")))

(event EventEndPlay
  (params (EndPlayReason :type EEndPlayReason%20Enum :default "Destroyed")))

(fn CheckforCameraCollisionZooming
  (params (Delta :type Float%20%28single-precision%29))
  (bind _distancetocheck (Variables|Default|GetDistanceToCheck))
  (bind _marucamera (Variables|Default|GetMaruCamera)
    (:then
      (bind _returnvalue (Collision|SphereTraceByChannel (Transformation|GetWorldLocation _marucamera) (+ (Transformation|GetWorldLocation _marucamera) (* (Math|Vector|GetForwardVector _marucamera) Delta _distancetocheck)) (/ _distancetocheck 2.0) "TraceTypeQuery2" false 0 "None"))
      (return _returnvalue))
    (:else)))

(fn CheckforCameraCollisionRotation
  (params (Quat :type Quat%20Structure))
  (bind (_x _y _z) (Class|KismetMathLibrary|BreakQuat Quat))
  (bind _distancetocheck (Variables|Default|GetDistanceToCheck))
  (bind _marucamera (Variables|Default|GetMaruCamera)
    (:then
      (bind _returnvalue (Collision|LineTraceByChannel (Transformation|GetWorldLocation _marucamera) (+ (Transformation|GetWorldLocation _marucamera) (* (* (Math|Vector|GetUpVector _marucamera) (- _x _y) (Math|Float|SelectFloat -3.0 3.0 (> (.yaw (Transformation|GetWorldRotation _marucamera)) 0.0))) _distancetocheck) (* (* (Math|Vector|GetRightVector _marucamera) _z -3.0) _distancetocheck)) "TraceTypeQuery2" false 0 "None"))
      (return _returnvalue))
    (:else)))

(fn CheckforCameraCollisionPanning
  (params (LocationDelta :type Vector))
  (bind _distancetocheck (Variables|Default|GetDistanceToCheck))
  (bind _marucamera (Variables|Default|GetMaruCamera)
    (:then
      (bind _returnvalue (Collision|SphereTraceByChannel (Transformation|GetWorldLocation _marucamera) (+ (Transformation|GetWorldLocation _marucamera) (* LocationDelta 2e+01 _distancetocheck)) (/ _distancetocheck 2.0) "TraceTypeQuery2" false 0 "None"))
      (return _returnvalue))
    (:else)))