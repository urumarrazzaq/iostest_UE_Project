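; BP_CameraPawn is a camera pawn driven by Enhanced Input look and zoom actions.
; IA_Look feeds its axes into controller pitch and yaw input.
; IA_Zoom scales the input and adjusts the SpringArm target arm length, clamped to a long-distance range.
; Both handlers print values to screen for debugging; BeginPlay, overlap and Tick are unused.
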(event Input|EnhancedActionEvents|EnhancedInputActionIA_Zoom
  (params (ActionValue :type Float%20%28double-precision%29) (ElapsedSeconds :type Float%20%28double-precision%29) (TriggeredSeconds :type Float%20%28double-precision%29) (InputAction :type Input%20Action%20Object%20Reference :default "/Game/ThirdPerson/Input/Actions/IA_Zoom.IA_Zoom"))
  (bind _springarm (Variables|Default|GetSpringArm))
  (Development|PrintString (Utilities|String|ToString(Float) (Math|Float|Clamp(Float) (+ (* ActionValue -1e+02) (Variables|/Script/Engine.SpringArmComponent|GetTargetArmLength _springarm)) 5e+03 1.5e+04)))
  (Variables|/Script/Engine.SpringArmComponent|SetTargetArmLength _springarm (Math|Float|Clamp(Float) (+ (* ActionValue -1e+02) (Variables|/Script/Engine.SpringArmComponent|GetTargetArmLength _springarm)) 5e+03 1.5e+04)))

(event Input|EnhancedActionEvents|EnhancedInputActionIA_Look
  (params (ActionValue :type Vector%202D%20Structure) (ElapsedSeconds :type Float%20%28double-precision%29) (TriggeredSeconds :type Float%20%28double-precision%29) (InputAction :type Input%20Action%20Object%20Reference :default "/Game/ThirdPerson/Input/Actions/IA_Look.IA_Look"))
  (bind (_x _y) (Math|Vector2D|BreakVector2D ActionValue))
  (Utilities|FlowControl|Sequence
    (:then_0
      (Pawn|Input|AddControllerPitchInput _y))
    (:then_1
      (Pawn|Input|AddControllerYawInput _x)
      (Development|PrintString (Utilities|String|ToString(Float) _x))
      (Development|PrintString (Utilities|String|ToString(Float) _y)))))

(event EventBeginPlay)

(event Collision|EventActorBeginOverlap
  (params (OtherActor :type Actor%20Object%20Reference)))

(event EventTick
  (params (DeltaSeconds :type Float%20%28single-precision%29)))

(fn ConstructionScript)