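; Player controller that handles touch selection of scene components, outlining the selected one through custom depth stencil.
; A first tap traced under the finger selects and starts a deselect timer; tapping it again zooms the BP_MyMaruCharacter camera to its owner.
; Missed taps deselect, and the character's UI ring release button, bound on possess, clears the outline.
; BeginPlay enables Slate global invalidation to cache UI.
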(event Custom|OnButtonRingsSeprate_Release
  ;[0.107 0.08228 0.2307] Remove the stencil on the selected object
  (CallFunction|ActivateCustomStencil))

(event EventBeginPlay
  ;[0.107 0.08228 0.2307] To Enable the Global Invalidation that will cache the ui to avoid multiple draw calls
  (Development|ExecuteConsoleCommand "Slate.EnableGlobalInvalidation 1" 0))

(event EventPossess
  (params (PossessedPawn :type Pawn%20Object%20Reference))
  ;[0.107 0.08228 0.2307] TODO: Change to something better relate to MyMaruCharacter
  (Utilities|FlowControl|DelayUntilNextTick)
  (bind _asbp_my_maru_character (Utilities|Casting|CastToBP_MyMaruCharacter PossessedPawn))
  (Utilities|IsValid (Variables|/Game/Blueprints/BP_MyMaruCharacter.BP_MyMaruCharacter_C|GetActiveUIRing _asbp_my_maru_character)
    (:Is%20Valid
      (Utilities|IsValid (Variables|/Game/UI/WBP_CurrencyUI.WBP_CurrencyUI_C|GetButtonRingsSeparate (Variables|/Game/Blueprints/BP_MyMaruCharacter.BP_MyMaruCharacter_C|GetActiveUIRing _asbp_my_maru_character))
        (:Is%20Valid
          (EventDispatchers|BindEventtoOnReleased (Variables|/Game/UI/WBP_CurrencyUI.WBP_CurrencyUI_C|GetButtonRingsSeparate (Variables|/Game/Blueprints/BP_MyMaruCharacter.BP_MyMaruCharacter_C|GetActiveUIRing _asbp_my_maru_character)) (EventDispatchers|CreateEvent :!event Custom|OnButtonRingsSeprate_Release)))))))

(event EventEndPlay
  (params (EndPlayReason :type EEndPlayReason%20Enum :default "Destroyed"))
  (bind _asbp_my_maru_character (Utilities|Casting|CastToBP_MyMaruCharacter (Game|Player|GetPlayerPawn 0)))
  (Utilities|IsValid (Variables|/Game/Blueprints/BP_MyMaruCharacter.BP_MyMaruCharacter_C|GetActiveUIRing _asbp_my_maru_character)
    (:Is%20Valid
      (Utilities|IsValid (Variables|/Game/UI/WBP_CurrencyUI.WBP_CurrencyUI_C|GetButtonRingsSeparate (Variables|/Game/Blueprints/BP_MyMaruCharacter.BP_MyMaruCharacter_C|GetActiveUIRing _asbp_my_maru_character))
        (:Is%20Valid
          (EventDispatchers|UnbindEventfromOnReleased (Variables|/Game/UI/WBP_CurrencyUI.WBP_CurrencyUI_C|GetButtonRingsSeparate (Variables|/Game/Blueprints/BP_MyMaruCharacter.BP_MyMaruCharacter_C|GetActiveUIRing _asbp_my_maru_character)) (EventDispatchers|CreateEvent :!event Custom|OnButtonRingsSeprate_Release)))))))

(fn ConstructionScript)

(fn ActivateCustomStencil
  (params (SelectedComponent :type Primitive%20Component%20Object%20Reference))
  (Utilities|FlowControl|Sequence
    (:then_0
      (Utilities|IsValid (Variables|Default|GetSelectedComponent)
        (:Is%20Valid
          (Rendering|SetRenderCustomDepth (Variables|Default|GetSelectedComponent) false)
          (Rendering|SetCustomDepthStencilValue (Variables|Default|GetSelectedComponent) 0))))
    (:then_1
      (Utilities|IsValid SelectedComponent
        (:Is%20Valid
          (Variables|Default|SetSelectedComponent SelectedComponent)
          (Rendering|SetRenderCustomDepth (Variables|Default|GetSelectedComponent) true)
          (Rendering|SetCustomDepthStencilValue (Variables|Default|GetSelectedComponent) 1))
        (:Is%20Not%20Valid
          (Variables|Default|SetSelectedComponent 0))))))

(fn TrySetSelectedComponent
  (bind (_hitresult _returnvalue) (Class|PlayerController|GetHitResultUnderFingerbyChannel "Touch1" "TraceTypeQuery3" true))
  (bind _selectedcomponent (Variables|Default|GetSelectedComponent))
  (bind _hitcomponent (Collision|BreakHitResult _hitresult))
  (bind _returnvalue_2 (Components|GetOwner _selectedcomponent))
  (bind _returnvalue_3 (Transformation|GetActorRotation _returnvalue_2))
  (bind _returnvalue_4 (Math|Rotator|CombineRotators _returnvalue_3 "-30.000000,180.000000,0.000000"))
  (bind _returnvalue_5 (Math|Conversions|ToQuaternion(Rotator) _returnvalue_4))
  (if _returnvalue
    (if (== _hitcomponent (Variables|Default|GetSelectedComponent))
      (bind _asbp_my_maru_character (Utilities|Casting|CastToBP_MyMaruCharacter (Game|Player|GetPlayerPawn 0)))
      (Variables|/Game/Blueprints/BP_MyMaruCharacter.BP_MyMaruCharacter_C|SetLast%20Active%20Object%20Location _asbp_my_maru_character (Utilities|Operators|Subtract (Transformation|GetActorLocation _returnvalue_2) (Class|MyMaruCharacter|GetCameraTarget _asbp_my_maru_character) "0.000000,0.000000,-60.000000"))
      (Variables|/Game/Blueprints/BP_MyMaruCharacter.BP_MyMaruCharacter_C|SetLast%20Active%20Object%20Rotation _asbp_my_maru_character _returnvalue_5)
      (Variables|/Game/Blueprints/BP_MyMaruCharacter.BP_MyMaruCharacter_C|SetbIsLastActiveObject? _asbp_my_maru_character true)
      (Class|MyMaruCharacter|SetCameraNewDistinction _asbp_my_maru_character (Utilities|Operators|Subtract (Transformation|GetActorLocation _returnvalue_2) (Class|MyMaruCharacter|GetCameraTarget _asbp_my_maru_character) "0.000000,0.000000,-60.000000") (Variables|Default|GetZoomingDistance) _returnvalue_5 2)
      (Utilities|Time|ClearandInvalidateTimerbyHandle (Variables|Default|GetDeselectTimerHandle))
      (Class|BPIInteract|SetZoomedin(Message) (Components|GetOwner (Variables|Default|GetSelectedComponent)) true)
      (else
        (CallFunction|ActivateCustomStencil _hitcomponent)
        (Class|BPIInteract|SetSelected(Message) (Components|GetOwner (Variables|Default|GetSelectedComponent)) true)
        (Utilities|Time|ClearandInvalidateTimerbyHandle (Variables|Default|GetDeselectTimerHandle))
        (bind _returnvalue_6 (Utilities|Time|SetTimerbyEvent (EventDispatchers|CreateEvent :!event DeselectComponent) (Variables|Default|GetDeselectTimer)))
        (Variables|Default|SetDeselectTimerHandle _returnvalue_6)))
    (else
      (CallFunction|DeselectComponent))))

(fn DeselectComponent
  (bind _selectedcomponent (Variables|Default|GetSelectedComponent))
  (Utilities|IsValid _selectedcomponent
    (:Is%20Valid
      (Class|BPIInteract|SetSelected(Message) (Components|GetOwner _selectedcomponent) false)
      (Class|BPIInteract|SetZoomedin(Message) (Components|GetOwner (Variables|Default|GetSelectedComponent)) false)
      (CallFunction|ActivateCustomStencil)
      (Utilities|Time|ClearandInvalidateTimerbyHandle (Variables|Default|GetDeselectTimerHandle)))))