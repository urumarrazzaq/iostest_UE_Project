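; BP_AIMaru is the AI-controlled Maru actor, which registers itself with the player's BP_MyMaruCharacter on BeginPlay.
; It feeds its behavior state to its AI controller's Blackboard, updating selection and zoom flags through setter events.
; Every tick it flags growth as in progress while GrowableRef is valid, and optionally snaps its yaw to face the player pawn when LookTowardPlayer is set.
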(event EventBeginPlay
  (bind _asbp_my_maru_character (Utilities|Casting|CastToBP_MyMaruCharacter (Game|Player|GetPlayerPawn 0)))
  (Variables|/Game/Blueprints/BP_MyMaruCharacter.BP_MyMaruCharacter_C|SetMaruAiActor _asbp_my_maru_character self))

(event EventTick
  (params (DeltaSeconds :type Float%20%28single-precision%29))
  (AI|Components|Blackboard|SetValueasBool (AI|GetBlackboard (AI|GetAIController self)) (Utilities|Name|MakeLiteralName "IsGrowthPhaseInProgress") (Utilities|IsValid (Variables|Default|GetGrowableRef)))
  (if (Variables|Default|GetLookTowardPlayer)
    (Transformation|SetActorRotation (Math|Rotator|MakeRotator 0.0 0.0 (.yaw (Math|Rotator|FindLookatRotation (Transformation|GetActorLocation) (Transformation|GetActorLocation (Game|Player|GetPlayerPawn 0))))))))

(event EventSetSelected
  (params (bIsSelected :type Boolean))
  (bind _output_get (Variables|Default|SetIs%20Selected bIsSelected))
  (AI|Components|Blackboard|SetValueasBool (AI|GetBlackboard (AI|GetAIController self)) (Utilities|Name|MakeLiteralName "HasBeenSelected") _output_get))

(event EventSetZoomedin
  (params (bIsZoomedIn :type Boolean))
  (bind _output_get (Variables|Default|SetIs%20Zoomed%20In bIsZoomedIn))
  (AI|Components|Blackboard|SetValueasBool (AI|GetBlackboard (AI|GetAIController self)) (Utilities|Name|MakeLiteralName "IsZoomed") _output_get))

(fn ConstructionScript)