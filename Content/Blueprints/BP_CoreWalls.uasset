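; Builds a procedural cross-section skirt of layered walls and a bottom face around a landscape, regenerated on construction and BeginPlay.
; Line traces along four edges, sized from a LandscapeComponent's bounds (square landscapes only), set each wall's top profile.
; Each layer's lower edge blends toward a target height with Perlin noise, clamped at the bottom, and seeds the next layer.
; Sections get planar UVs and per-layer materials.
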(event Custom|GenerateWalls
  (bind _proceduralmesh (Variables|Default|GetProceduralMesh))
  (bind _layermaterials (Variables|Default|GetLayerMaterials))
  (bind _proceduralmesh_2 (Variables|Default|GetProceduralMesh))
  (bind _landscaperef (Variables|Default|GetLandscapeRef))
  (bind _proceduralmesh_3 (Variables|Default|GetProceduralMesh))
  (bind _bottomheight (Variables|Default|GetBottomHeight))
  (bind _returnvalue (Transformation|GetActorLocation _landscaperef))
  (Class|ProceduralMeshComponent|ClearAllMeshSections (Variables|Default|GetProceduralMesh))
  ;[0.15 0.15 0.15 0.5] Get side length using Landscape Component Bounds
  ; ###WILL NOT WORK FOR NON-SQUARE LANDSCAPES###
  (Variables|Default|SetSideLength (.x (.BoxExtent (Collision|GetComponentBounds (Actor|GetComponentbyClass (Variables|Default|GetLandscapeRef) "/Script/Landscape.LandscapeComponent"))))) ; Only works on a landscape with uniform sides
  ;[0.15 0.15 0.15 0.5] Create Mesh Sections for 4 Side Walls
  (for _index (range 0 3) ; Walls
    (Utilities|Array|Clear (Variables|Default|GetBottomVertices))
    (for _index_2 (range 0 (Utilities|Array|LastIndex (Variables|Default|GetLayerMaterials))) ; Layers
      (Utilities|Array|Clear (Variables|Default|GetVertices))
      (if (Utilities|Array|IsEmpty (Variables|Default|GetBottomVertices))
        ;;[0.15 0.15 0.15 0.5] If Top Layer, Use Line Traces with a set resolution (Trace Resolution) to set the top edge vertices
        (for _index_3 (range 0 (Variables|Default|GetTraceResolution))
          (bind _outhit (Collision|LineTraceForObjects (Math|Vector|MakeVector (.x (CallFunction|GetTraceLocation2D _index _index_3)) (.y (CallFunction|GetTraceLocation2D _index _index_3)) (Variables|Default|GetBottomHeight)) (Math|Vector|MakeVector (.x (CallFunction|GetTraceLocation2D _index _index_3)) (.y (CallFunction|GetTraceLocation2D _index _index_3)) 1e+03) (Utilities|Array|MakeArray "ObjectTypeQuery1") true (Variables|Default|GetTraceIgnoreActors) "None" true "(R=1.000000,G=0.000000,B=0.000000,A=1.000000)" "(R=0.000000,G=1.000000,B=0.000000,A=1.000000)" 2.0))
          (Utilities|Array|Add (Variables|Default|GetVertices) (.Location (Collision|BreakHitResult _outhit))))
        (else
          (Variables|Default|SetVertices (Variables|Default|GetBottomVertices))
          (Utilities|Array|Clear (Variables|Default|GetBottomVertices))))
      ;;[0.15 0.15 0.15 0.5] Set Bottom Edge Vertices and append to Top Edge Vertices
      (for _array_element (Variables|Default|GetVertices)
        (Utilities|Array|Add (Variables|Default|GetBottomVertices) (Math|Vector|MakeVector (.x _array_element) (.y _array_element) (Math|Float|Max(Float) (+ (- (.z _array_element) (* (- (.z _array_element) (Utilities|Array|Get(acopy) (Variables|Default|GetLayerDesiredBottomZHeights) _index_2)) (Utilities|Array|Get(acopy) (Variables|Default|GetLayerDepthScalars) _index_2))) (.z (Class|KismetAnimationLibrary|MakePerlinNoiseVectorandRemap (.x (* (Math|Vector|MakeVector (.x _array_element) (.y _array_element) (- (.z _array_element) (* (- (.z _array_element) (Utilities|Array|Get(acopy) (Variables|Default|GetLayerDesiredBottomZHeights) _index_2)) (Utilities|Array|Get(acopy) (Variables|Default|GetLayerDepthScalars) _index_2)))) (Variables|Default|GetNoiseFrequency))) (.y (* (Math|Vector|MakeVector (.x _array_element) (.y _array_element) (- (.z _array_element) (* (- (.z _array_element) (Utilities|Array|Get(acopy) (Variables|Default|GetLayerDesiredBottomZHeights) _index_2)) (Utilities|Array|Get(acopy) (Variables|Default|GetLayerDepthScalars) _index_2)))) (Variables|Default|GetNoiseFrequency))) (.z (* (Math|Vector|MakeVector (.x _array_element) (.y _array_element) (- (.z _array_element) (* (- (.z _array_element) (Utilities|Array|Get(acopy) (Variables|Default|GetLayerDesiredBottomZHeights) _index_2)) (Utilities|Array|Get(acopy) (Variables|Default|GetLayerDepthScalars) _index_2)))) (Variables|Default|GetNoiseFrequency))) "-1.f" "1.f" "-1.f" "1.f" (* (* (Utilities|Array|Get(acopy) (Variables|Default|GetLayerNoiseScalars) _index_2) 1e+02) -1.0) (* (Utilities|Array|Get(acopy) (Variables|Default|GetLayerNoiseScalars) _index_2) 1e+02)))) (Variables|Default|GetBottomHeight)))))
      (Utilities|Array|AppendArray (Variables|Default|GetVertices) (Variables|Default|GetBottomVertices))
      ;;[0.15 0.15 0.15 0.5] Generate Triangles Array
      (Utilities|Array|Clear (Variables|Default|GetTriangles))
      (for _index_4 (range 0 (- (- (Utilities|Array|Length (Variables|Default|GetVertices)) (Utilities|Array|Length (Variables|Default|GetBottomVertices))) 2))
        (Utilities|Array|Add (Variables|Default|GetTriangles) _index_4)
        (Utilities|Array|Add (Variables|Default|GetTriangles) (+ _index_4 (- (Utilities|Array|Length (Variables|Default|GetVertices)) (Utilities|Array|Length (Variables|Default|GetBottomVertices))) 1))
        (Utilities|Array|Add (Variables|Default|GetTriangles) (+ (- (Utilities|Array|Length (Variables|Default|GetVertices)) (Utilities|Array|Length (Variables|Default|GetBottomVertices))) _index_4))
        (Utilities|Array|Add (Variables|Default|GetTriangles) _index_4)
        (Utilities|Array|Add (Variables|Default|GetTriangles) (+ _index_4 1))
        (Utilities|Array|Add (Variables|Default|GetTriangles) (+ _index_4 (- (Utilities|Array|Length (Variables|Default|GetVertices)) (Utilities|Array|Length (Variables|Default|GetBottomVertices))) 1)))
      (Class|ProceduralMeshComponent|CreateMeshSectionLinearColor _proceduralmesh_3 (Class|ProceduralMeshComponent|GetNumSections _proceduralmesh_3) (Variables|Default|GetVertices) (Variables|Default|GetTriangles) 0 (CallFunction|GenerateUVs (Variables|Default|GetVertices) _index_2) 0 0 0 0 0 false false)))
  ;[0.15 0.15 0.15 0.5] Create Bottom Mesh Section
  (Utilities|Array|Clear (Variables|Default|GetVertices))
  (Utilities|Array|Clear (Variables|Default|GetTriangles))
  (Variables|Default|SetVertices (Utilities|Array|MakeArray (Math|Vector|MakeVector (.x _returnvalue) (.y _returnvalue) _bottomheight) (Math|Vector|MakeVector (+ (.x _returnvalue) (* (Variables|Default|GetSideLength) 2.0)) (.y _returnvalue) _bottomheight) (Math|Vector|MakeVector (+ (.x _returnvalue) (* (Variables|Default|GetSideLength) 2.0)) (+ (.y _returnvalue) (* (Variables|Default|GetSideLength) 2.0)) _bottomheight) (Math|Vector|MakeVector (.x _returnvalue) (+ (.y _returnvalue) (* (Variables|Default|GetSideLength) 2.0)) _bottomheight)))
  (for _index_5 (range 0 (- (Utilities|Array|Length (Variables|Default|GetVertices)) 2))
    (Utilities|Array|Add (Variables|Default|GetTriangles) _index_5)
    (Utilities|Array|Add (Variables|Default|GetTriangles) (+ _index_5 (Utilities|Array|Length (Variables|Default|GetVertices)) 1))
    (Utilities|Array|Add (Variables|Default|GetTriangles) (+ (Utilities|Array|Length (Variables|Default|GetVertices)) _index_5))
    (Utilities|Array|Add (Variables|Default|GetTriangles) _index_5)
    (Utilities|Array|Add (Variables|Default|GetTriangles) (+ _index_5 1))
    (Utilities|Array|Add (Variables|Default|GetTriangles) (+ _index_5 (Utilities|Array|Length (Variables|Default|GetVertices)) 1)))
  (Class|ProceduralMeshComponent|CreateMeshSectionLinearColor _proceduralmesh_2 (Class|ProceduralMeshComponent|GetNumSections _proceduralmesh_2) (Variables|Default|GetVertices) (Variables|Default|GetTriangles) 0 (CallFunction|GenerateUVs (Variables|Default|GetVertices) _index_2) 0 0 0 0 0 false false)
  ;[0.15 0.15 0.15 0.5] Set Material for all Mesh Sections
  (for _index_6 (range 0 (+ (Class|ProceduralMeshComponent|GetNumSections (Variables|Default|GetProceduralMesh)) 1))
    (Rendering|Material|SetMaterial (Variables|Default|GetProceduralMesh) _index_6 (Utilities|Array|Get(acopy) _layermaterials (Math|Integer|%(Integer) _index_6 (Utilities|Array|Length _layermaterials)))))
  (Rendering|Material|SetMaterial _proceduralmesh (+ (Class|ProceduralMeshComponent|GetNumSections _proceduralmesh) -1) (Variables|Default|GetBottomMaterial))
  (Rendering|SetBoundsScale (Variables|Default|GetProceduralMesh) 1e+01) ; To make sure mesh isn't culled
)

(event EventBeginPlay
  (CallFunction|GenerateWalls))

(fn ConstructionScript
  (CallFunction|GenerateWalls))

(fn GetTraceLocation2D
  (params (FaceIndex :type Integer) (TraceIndex :type Integer))
  (bind _landscaperef (Variables|Default|GetLandscapeRef))
  (bind _sidelength (Variables|Default|GetSideLength))
  (bind _sidelength_2 (Variables|Default|GetSideLength))
  (bind _landscaperef_2 (Variables|Default|GetLandscapeRef))
  (bind _landscaperef_3 (Variables|Default|GetLandscapeRef))
  (bind _landscaperef_4 (Variables|Default|GetLandscapeRef))
  (bind _returnvalue (Transformation|GetActorLocation _landscaperef_2))
  (bind _returnvalue_2 (Transformation|GetActorLocation _landscaperef_3))
  (bind _returnvalue_3 (Transformation|GetActorLocation _landscaperef_4))
  (bind _returnvalue_4 (Transformation|GetActorLocation _landscaperef))
  (bind _returnvalue_5 (* _sidelength 2.0))
  (bind _returnvalue_6 (* _sidelength_2 2.0))
  (switch int FaceIndex
    (:0
      (return (Math|Vector2D|MakeVector2D (+ (.x _returnvalue_3) (* (/ (* (Variables|Default|GetSideLength) 2.0) (Variables|Default|GetTraceResolution)) TraceIndex)) (.y _returnvalue_3))))
    (:1
      (return (Math|Vector2D|MakeVector2D (.x _returnvalue_2) (+ (* (/ (* (Variables|Default|GetSideLength) 2.0) (Variables|Default|GetTraceResolution)) TraceIndex -1.0) (.y _returnvalue_2) (* (Variables|Default|GetSideLength) 2.0)))))
    (:2
      (return (Math|Vector2D|MakeVector2D (+ (.x _returnvalue_4) _returnvalue_5) (+ (* (/ _returnvalue_5 (Variables|Default|GetTraceResolution)) TraceIndex) (.y _returnvalue_4)))))
    (:3
      (return (Math|Vector2D|MakeVector2D (+ (.x _returnvalue) _returnvalue_6 (* (/ _returnvalue_6 (Variables|Default|GetTraceResolution)) -1.0 TraceIndex)) (+ _returnvalue_6 (.y _returnvalue)))))))

(fn GenerateUVs
  (params (Vertices :type Array%20of%20Vectors) (Layer :type Integer))
  (bind _output (Utilities|Array|Get(acopy) Vertices 1))
  (bind _output_2 (Utilities|Array|Get(acopy) Vertices))
  (bind _returnvalue (- _output_2 _output))
  (LocalVariables|SetTextureScale (Utilities|Array|Get(acopy) (Variables|Default|GetLayerTextureScale) Layer))
  (if (!= (.y _returnvalue) 0.0)
    (for _array_element Vertices
      (Utilities|Array|Add (LocalVariables|GetUVs) (Math|Vector2D|MakeVector2D (/ (.y _array_element) (LocalVariables|GetTextureScale)) (/ (.z _array_element) (LocalVariables|GetTextureScale)))))
    (return (LocalVariables|GetUVs))
    (elif (!= (.z _returnvalue) 0.0)
      (for _array_element_2 Vertices
        (Utilities|Array|Add (LocalVariables|GetUVs) (Math|Vector2D|MakeVector2D (/ (.x _array_element_2) (LocalVariables|GetTextureScale)) (/ (.z _array_element_2) (LocalVariables|GetTextureScale)))))
      (return (LocalVariables|GetUVs))
      (else
        (for _array_element_3 Vertices
          (Utilities|Array|Add (LocalVariables|GetUVs) (Math|Vector2D|MakeVector2D (/ (.x _array_element_3) (LocalVariables|GetTextureScale)) (/ (.y _array_element_3) (LocalVariables|GetTextureScale)))))
        (return (LocalVariables|GetUVs))))))