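; Butterfly actor that flies autonomously with a random texture and offset flap animation.
; Tick dispatches a behavior-state machine: gliding, slow/fast turning and obstacle avoidance set target rotation using Perlin wobble and weighted random exits, while other states are stubs.
; Rotation interpolates toward that target, and flying states sweep-move forward at pitch-dependent speed.
; A forward box trace triggers avoidance, which tests random rotations for a clear path.
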(event Custom|LandedTick)

(event Custom|LandingTick)

(event Custom|TurningFastTick
  (bind _returnvalue (Transformation|GetActorLocation))
  ;[0.15 0.15 0.15 0.5] Turning Slow AND Turning Fast Tick Events
  (Variables|Default|SetRotationSpeed (* (Utilities|GetClassDefaults "BP_Butterfly_C") 4.0))
  (if (or (Utilities|Enum|Equal(Enum) (Variables|Default|GetTurningDirection) "Left") (Utilities|Enum|Equal(Enum) (Variables|Default|GetTurningDirection) "Right")) ; If turning direction isnt already set to left or right, randomly set it to one of them
    _
    (else
      (Variables|Default|SetTurningDirection (select (Math|Random|RandomBool) "Right" "Left"))))
  ;;[0.15 0.15 0.15 0.5] Set target rotation to rotate towards a point that's in front of me but to one side but override roll to wobble around a set number
  (Variables|Default|SetTargetRotation (Math|Rotator|MakeRotator (+ (* 6e+01 (- (* (Math|Conversions|ToInteger(Boolean) (Utilities|Enum|Equal(Enum) (Variables|Default|GetTurningDirection) "Left")) 2) 1)) (* (Class|KismetMathLibrary|PerlinNoise1D (+ (* (Actor|GetGameTimeSinceCreation) 1.4) 0.0)) 5.0 (+ (Math|Conversions|ToInteger(Boolean) (Utilities|Enum|Equal(Enum) (Variables|Default|GetBehaviorState) "NewEnumerator9")) 1))) (+ (.pitch (Math|Rotator|FindLookatRotation _returnvalue (+ _returnvalue (* (Transformation|GetActorForwardVector) 5e+01) (* (Transformation|GetActorUpVector) 7e+01) (* (Transformation|GetActorRightVector) 5e+01 (- (* (Math|Conversions|ToInteger(Boolean) (Utilities|Enum|Equal(Enum) (Variables|Default|GetTurningDirection) "Left")) 2) 1))))) (* (Class|KismetMathLibrary|PerlinNoise1D (+ (* (Actor|GetGameTimeSinceCreation) 1.4) 5e+02)) 5.0 (+ (Math|Conversions|ToInteger(Boolean) (Utilities|Enum|Equal(Enum) (Variables|Default|GetBehaviorState) "NewEnumerator9")) 1))) (+ (.yaw (Math|Rotator|FindLookatRotation _returnvalue (+ _returnvalue (* (Transformation|GetActorForwardVector) 5e+01) (* (Transformation|GetActorUpVector) 7e+01) (* (Transformation|GetActorRightVector) 5e+01 (- (* (Math|Conversions|ToInteger(Boolean) (Utilities|Enum|Equal(Enum) (Variables|Default|GetTurningDirection) "Left")) 2) 1))))) (* (Class|KismetMathLibrary|PerlinNoise1D (+ (* (Actor|GetGameTimeSinceCreation) 1.4) 1e+03)) 5.0 (+ (Math|Conversions|ToInteger(Boolean) (Utilities|Enum|Equal(Enum) (Variables|Default|GetBehaviorState) "NewEnumerator9")) 1)))))
  ;;[0.05098 0.149 0.02353 0.502] Exit Condition
  (if (Math|Random|RandomBoolwithWeight (Math|Float|SelectFloat (Math|Float|MapRangeClamped (Variables|Default|GetTimeSpentInCurrentState) 0.4 3.5 0.01 0.03) (Math|Float|MapRangeClamped (Variables|Default|GetTimeSpentInCurrentState) 1.0 3.5 0.01 0.03) (Utilities|Enum|Equal(Enum) (Variables|Default|GetBehaviorState) "NewEnumerator10")))
    (Variables|Default|SetBehaviorState (.OutItem (Utilities|Array|Random (Variables|Default|GetFlyingStates))))
    (Variables|Default|SetTurningDirection "Back") ; Having this here handles the case where we switch directly between turning states (allows the direction to be re-rolled)
  ))

(event Custom|RandomizeRotation
  (bind _returnvalue (Transformation|GetActorRotation))
  (Transformation|SetActorRotation (Math|Rotator|MakeRotator (.roll _returnvalue) (.pitch _returnvalue) (Math|Random|RandomFloatinRange 0.0 3.6e+02))))

(event Custom|TakingOffTick)

(event Custom|GlidingTick
  ;[0.15 0.15 0.15 0.5] Gliding Tick Event
  ;;[0.15 0.15 0.15 0.5] Set target rotation to flat + some wobble
  (Variables|Default|SetTargetRotation (Math|Rotator|MakeRotator (* (Class|KismetMathLibrary|PerlinNoise1D (* (Actor|GetGameTimeSinceCreation) 1.4)) 35.0) (* (Class|KismetMathLibrary|PerlinNoise1D (+ (* (Actor|GetGameTimeSinceCreation) 1.4) 5e+02)) 35.0) (+ (* (Class|KismetMathLibrary|PerlinNoise1D (Actor|GetGameTimeSinceCreation)) 2e+01) (.yaw (Transformation|GetActorRotation)))))
  (Variables|Default|SetRotationSpeed (Utilities|GetClassDefaults "BP_Butterfly_C"))
  ;;[0.05098 0.149 0.02353 0.502] Exit Condition
  (if (Math|Random|RandomBoolwithWeight (Math|Float|MapRangeClamped (Variables|Default|GetTimeSpentInCurrentState) 2.0 7.0 0.01 0.03))
    (Variables|Default|SetBehaviorState (.OutItem (Utilities|Array|Random (Variables|Default|GetFlyingStates))))))

(event Custom|ClimbingTick)

(event Custom|AvoidingObstacleTick
  ;[0.15 0.15 0.15 0.5] Avoiding Obstacle Tick Event
  (if (Utilities|Operators|NotEqual(!=) :A (Variables|Default|GetAvoidObstacleTarget))
    (if (< (+ (.roll (Math|Rotator|Delta(Rotator) (Transformation|GetActorRotation) (Variables|Default|GetAvoidObstacleTarget))) (.pitch (Math|Rotator|Delta(Rotator) (Transformation|GetActorRotation) (Variables|Default|GetAvoidObstacleTarget))) (.yaw (Math|Rotator|Delta(Rotator) (Transformation|GetActorRotation) (Variables|Default|GetAvoidObstacleTarget)))) 2e+01) ; Keep rotating towards the AvoidObstacleTarget until within a certain threshold, then unset the AvoidObstacleTarget
      (Variables|Default|SetAvoidObstacleTarget "0, 0, 0")
      (else
        (Variables|Default|SetTargetRotation (Variables|Default|GetAvoidObstacleTarget))
        (Variables|Default|SetRotationSpeed (* (Utilities|GetClassDefaults "BP_Butterfly_C") 3.0))))
    (else
      ;;[0.05246 0.15 0.02516 0.5] Exit Condition
      (if (CallFunction|IsThereAnObstacleinFrontOfMe)
        (bind (_success _rotation) (CallFunction|WhatDirectionHasNoObstacles))
        (if _success
          (Variables|Default|SetTargetRotation _rotation)
          (else
            (Variables|Default|SetAvoidObstacleTarget "0, 0, 0")))
        (else
          (Variables|Default|SetAvoidObstacleTarget "0, 0, 0")
          (Variables|Default|SetBehaviorState (.OutItem (Utilities|Array|Random (Variables|Default|GetFlyingStates)))))))))

(event Custom|HangingTick)

(event Custom|DippingTick)

(event Custom|HoppingTick)

(event Custom|TurningSlowTick
  (bind _returnvalue (Transformation|GetActorLocation))
  ;[0.15 0.15 0.15 0.5] Turning Slow AND Turning Fast Tick Events
  (Variables|Default|SetRotationSpeed (* (Utilities|GetClassDefaults "BP_Butterfly_C") 2.0))
  (if (or (Utilities|Enum|Equal(Enum) (Variables|Default|GetTurningDirection) "Left") (Utilities|Enum|Equal(Enum) (Variables|Default|GetTurningDirection) "Right")) ; If turning direction isnt already set to left or right, randomly set it to one of them
    _
    (else
      (Variables|Default|SetTurningDirection (select (Math|Random|RandomBool) "Right" "Left"))))
  ;;[0.15 0.15 0.15 0.5] Set target rotation to rotate towards a point that's in front of me but to one side but override roll to wobble around a set number
  (Variables|Default|SetTargetRotation (Math|Rotator|MakeRotator (+ (* 6e+01 (- (* (Math|Conversions|ToInteger(Boolean) (Utilities|Enum|Equal(Enum) (Variables|Default|GetTurningDirection) "Left")) 2) 1)) (* (Class|KismetMathLibrary|PerlinNoise1D (+ (* (Actor|GetGameTimeSinceCreation) 1.4) 0.0)) 5.0 (+ (Math|Conversions|ToInteger(Boolean) (Utilities|Enum|Equal(Enum) (Variables|Default|GetBehaviorState) "NewEnumerator9")) 1))) (+ (.pitch (Math|Rotator|FindLookatRotation _returnvalue (+ _returnvalue (* (Transformation|GetActorForwardVector) 5e+01) (* (Transformation|GetActorUpVector) 7e+01) (* (Transformation|GetActorRightVector) 5e+01 (- (* (Math|Conversions|ToInteger(Boolean) (Utilities|Enum|Equal(Enum) (Variables|Default|GetTurningDirection) "Left")) 2) 1))))) (* (Class|KismetMathLibrary|PerlinNoise1D (+ (* (Actor|GetGameTimeSinceCreation) 1.4) 5e+02)) 5.0 (+ (Math|Conversions|ToInteger(Boolean) (Utilities|Enum|Equal(Enum) (Variables|Default|GetBehaviorState) "NewEnumerator9")) 1))) (+ (.yaw (Math|Rotator|FindLookatRotation _returnvalue (+ _returnvalue (* (Transformation|GetActorForwardVector) 5e+01) (* (Transformation|GetActorUpVector) 7e+01) (* (Transformation|GetActorRightVector) 5e+01 (- (* (Math|Conversions|ToInteger(Boolean) (Utilities|Enum|Equal(Enum) (Variables|Default|GetTurningDirection) "Left")) 2) 1))))) (* (Class|KismetMathLibrary|PerlinNoise1D (+ (* (Actor|GetGameTimeSinceCreation) 1.4) 1e+03)) 5.0 (+ (Math|Conversions|ToInteger(Boolean) (Utilities|Enum|Equal(Enum) (Variables|Default|GetBehaviorState) "NewEnumerator9")) 1)))))
  ;;[0.05098 0.149 0.02353 0.502] Exit Condition
  (if (Math|Random|RandomBoolwithWeight (Math|Float|SelectFloat (Math|Float|MapRangeClamped (Variables|Default|GetTimeSpentInCurrentState) 0.4 3.5 0.01 0.03) (Math|Float|MapRangeClamped (Variables|Default|GetTimeSpentInCurrentState) 1.0 3.5 0.01 0.03) (Utilities|Enum|Equal(Enum) (Variables|Default|GetBehaviorState) "NewEnumerator10")))
    (Variables|Default|SetBehaviorState (.OutItem (Utilities|Array|Random (Variables|Default|GetFlyingStates))))
    (Variables|Default|SetTurningDirection "Back") ; Having this here handles the case where we switch directly between turning states (allows the direction to be re-rolled)
  ))

(event EventBeginPlay
  (Components|Animation|SetPosition (Variables|Default|GetButterflyMesh) (Math|Random|RandomFloatinRange 1.0 5.0) false) ; Randomly offsets start position of flying animation so wings aren't all synced
  ;[0.15 0.15 0.15 0.5] Assign a random texture from the set within the material
  (bind _returnvalue (Rendering|Material|CreateDynamicMaterialInstance (Variables|Default|GetButterflyMesh) 0 "/Game/Blueprints/Butterfly/M_Butterfly.M_Butterfly" "None" :!class /Script/Engine.PrimitiveComponent))
  (Rendering|Material|SetScalarParameterValue _returnvalue "TextureIndex" (Math|Conversions|ToFloat(Integer) (Math|Float|Round (Math|Random|RandomFloatinRange 0.0 1e+01))) :!class /Script/Engine.MaterialInstanceDynamic)
  (Rendering|Material|SetMaterial (Variables|Default|GetButterflyMesh) 0 _returnvalue)
  (Variables|Default|SetPreviousBehaviorState (Variables|Default|GetBehaviorState)))

(event EventTick
  (params (DeltaSeconds :type Float%20%28single-precision%29))
  (bind _returnvalue (Transformation|GetActorForwardVector))
  (bind _returnvalue_2 (Transformation|GetActorLocation))
  ;[0.05286 0.15 0.02519 0.502] If flying, check if there is an obstacle in front of me, if there is then set my state to Avoiding Obstacle
  ; ### ACTS AS AN EXIT CONDITION FOR ALL FLYING STATES ###
  (if (and (Utilities|Array|ContainsItem (Variables|Default|GetFlyingStates) (Variables|Default|GetBehaviorState)) (Utilities|Enum|NotEqual(Enum) (Variables|Default|GetBehaviorState) "NewEnumerator5"))
    (if (CallFunction|IsThereAnObstacleinFrontOfMe)
      (Variables|Default|SetBehaviorState "NewEnumerator5")))
  ;[0.15 0.15 0.15 0.5] If behavior state is not Turning, set turn direction to not left or right (allows turn direction to be determined randomly when turning state is entered for the first time)
  (if (Math|Boolean|NORBoolean (Utilities|Enum|Equal(Enum) (Variables|Default|GetBehaviorState) "NewEnumerator9") (Utilities|Enum|Equal(Enum) (Variables|Default|GetBehaviorState) "NewEnumerator10"))
    (Variables|Default|SetTurningDirection "Back"))
  ;[0.15 0.15 0.15 0.5] Check if the behavior state changed since last tick and update Time Spent in Current State
  (if (Utilities|Enum|Equal(Enum) (Variables|Default|GetBehaviorState) (Variables|Default|GetPreviousBehaviorState))
    (Variables|Default|SetTimeSpentInCurrentState (+ (Variables|Default|GetTimeSpentInCurrentState) (Utilities|Time|GetWorldDeltaSeconds)))
    (else
      (Variables|Default|SetTimeSpentInCurrentState 0.0)))
  (Variables|Default|SetPreviousBehaviorState (Variables|Default|GetBehaviorState))
  (if (Variables|Default|GetShow) ; DEBUG- Print current behavior state
    (Development|PrintString (Utilities|String|EnumtoString (Variables|Default|GetBehaviorState)) true true "(R=0.000000,G=0.660000,B=1.000000,A=1.000000)" 0.0))
  (switch Utilities|FlowControl|Switch|SwitchonE_ButterflyBehaviorState (Variables|Default|GetBehaviorState)
    (:NewEnumerator0
      (|ExecuteBehaviorStateTickEvents :!label _label)
      (if (Variables|Default|GetShow) ; DEBUG- Draw line that shows current target rotation
        (Rendering|Debug|DrawDebugLine _returnvalue_2 (+ _returnvalue_2 (* (Math|Rotator|GetRotationXVector (Variables|Default|GetTargetRotation)) 3e+02)) "(R=0.000000,G=0.173304,B=1.000000,A=1.000000)" 0.0 1e+01))
      (Transformation|SetActorRotation (Class|KismetMathLibrary|RInterptoConstant (Transformation|GetActorRotation) (Variables|Default|GetTargetRotation) (Utilities|Time|GetWorldDeltaSeconds) (* (Variables|Default|GetRotationSpeed) (Math|Float|MapRangeClamped (Class|KismetMathLibrary|PerlinNoise1D (Actor|GetGameTimeSinceCreation)) -1.0 1.0 0.8 1.2) (Math|Float|Max(Float) (Math|Float|MapRangeUnclamped (Class|KismetMathLibrary|DegAtan2 (.z _returnvalue) (Math|Vector|VectorLength (Math|Vector|MakeVector (.x _returnvalue) (.y _returnvalue) 0.0))) -4e+01 4e+01 2.0 0.7) 0.7))))
      (if (Utilities|Array|ContainsItem (Variables|Default|GetFlyingStates) (Variables|Default|GetBehaviorState))
        (CallFunction|UpdateMoveSpeed)
        (Variables|Default|SetMoveDirection (Transformation|GetActorForwardVector))
        (Transformation|AddActorWorldOffset (* (Variables|Default|GetMoveDirection) (Variables|Default|GetMoveSpeed) 1.0) true)))
    (:NewEnumerator1
      (goto _label Landing))
    (:NewEnumerator2
      (goto _label TakingOff))
    (:NewEnumerator3
      (goto _label Gliding))
    (:NewEnumerator4
      (goto _label Climbing))
    (:NewEnumerator5
      (goto _label AvoidingObstacle))
    (:NewEnumerator6
      (goto _label Hanging))
    (:NewEnumerator7
      (goto _label Dipping))
    (:NewEnumerator8
      (goto _label Hopping))
    (:NewEnumerator9
      (goto _label TurningSlow))
    (:NewEnumerator10
      (goto _label TurningFast))))

(fn ConstructionScript)

(fn IsThereAnObstacleinFrontOfMe
  (bind _returnvalue (Transformation|GetActorLocation))
  (bind _butterflymesh (Variables|Default|GetButterflyMesh))
  (bind _relativescale3d (Variables|/Script/Engine.SceneComponent|GetRelativeScale3D _butterflymesh))
  (bind _returnvalue_2 (* (.x _relativescale3d) 5e+01))
  (bind _returnvalue_3 (Collision|BoxTraceByChannel _returnvalue (+ _returnvalue (* (Math|Vector|Normalize (Variables|Default|GetMoveDirection)) (LocalVariables|GetTestDistance) (.x _relativescale3d))) (Math|Vector|MakeVector _returnvalue_2 _returnvalue_2 _returnvalue_2) "0, 0, 0" "TraceTypeQuery1" false 0 (select (Variables|Default|GetShow) "ForOneFrame" "None")))
  (return _returnvalue_3))

(fn WhatDirectionHasNoObstacles
  (bind _returnvalue (Transformation|GetActorLocation))
  (bind _butterflymesh (Variables|Default|GetButterflyMesh))
  (bind _relativescale3d (Variables|/Script/Engine.SceneComponent|GetRelativeScale3D _butterflymesh))
  (bind _returnvalue_2 (* (.x _relativescale3d) 6e+01))
  (bind _index (Utilities|FlowControl|ForLoopwithBreak 10 40 :!label _label)
    (:LoopBody
      (LocalVariables|SetTestRotation (Math|Rotator|CombineRotators (Math|Rotator|FindLookatRotation _returnvalue (+ _returnvalue (Variables|Default|GetMoveDirection))) (* (Math|Random|RandomRotator false) (* _index 0.02 (- (* (Math|Conversions|ToInteger(Boolean) (Math|Random|RandomBool)) 2) 1)))))
      (bind _returnvalue_3 (Collision|BoxTraceByChannel (+ _returnvalue (* (Math|Rotator|GetRotationXVector (LocalVariables|GetTestRotation)) 1e+02)) (+ _returnvalue (* (Math|Rotator|GetRotationXVector (LocalVariables|GetTestRotation)) (LocalVariables|GetTestDistance) (.x _relativescale3d))) (Math|Vector|MakeVector _returnvalue_2 _returnvalue_2 _returnvalue_2) "0, 0, 0" "TraceTypeQuery1" false 0 "None" true "(R=0.967998,G=1.000000,B=0.000000,A=1.000000)" "(R=0.857027,G=0.000000,B=1.000000,A=1.000000)"))
      (if (not _returnvalue_3)
        (Variables|Default|SetAvoidObstacleTarget (LocalVariables|GetTestRotation))
        (LocalVariables|SetTestSucceeded true)
        (goto _label Break)))
    (:Completed
      (return (LocalVariables|GetTestSucceeded) (Variables|Default|GetAvoidObstacleTarget)))))

(fn LookforLandingSpot
  (return false "0, 0, 0" "0, 0, 0"))

(fn UpdateMoveSpeed
  (bind _returnvalue (Transformation|GetActorForwardVector))
  (bind _movespeed (Utilities|GetClassDefaults "BP_Butterfly_C"))
  (LocalVariables|SetTargetSpeed (Math|Float|MapRangeUnclamped (Class|KismetMathLibrary|DegAtan2 (.z _returnvalue) (Math|Vector|VectorLength (Math|Vector|MakeVector (.x _returnvalue) (.y _returnvalue) 0.0))) -4e+01 4e+01 (* _movespeed 2.0) (* _movespeed 0.5)))
  (Variables|Default|SetMoveSpeed (Math|Interpolation|FInterptoConstant (Variables|Default|GetMoveSpeed) (LocalVariables|GetTargetSpeed) (Utilities|Time|GetWorldDeltaSeconds) (Math|Float|SelectFloat 0.7 2.0 (> (Variables|Default|GetMoveSpeed) (LocalVariables|GetTargetSpeed)))))
  (return))