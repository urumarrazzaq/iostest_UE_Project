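; BP_CandleOnOff is a sphere trigger that lights or blows out any BP_Candle actor that begins overlapping it.
; The LightCandles flag chooses between calling CandleLit and BlownOut on the candle.
; Each call passes a random delay up to RandomDelayAmount, so groups of candles change staggered rather than all at once.
; The construction script sets the sphere size from SphereRadius.
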(event OnComponentBeginOverlap(Sphere)
  (params (OverlappedComponent :type Primitive%20Component%20Object%20Reference) (OtherActor :type Actor%20Object%20Reference) (OtherComp :type Primitive%20Component%20Object%20Reference) (OtherBodyIndex :type Integer) (bFromSweep :type Boolean) (SweepResult :type Hit%20Result%20Structure%20%28by%20ref%29))
  (bind _randomdelayamount (Variables|Default|GetRandomDelayAmount))
  (bind _returnvalue (Math|Random|RandomFloatinRange 0.0 _randomdelayamount))
  (bind _asbp_candle (Utilities|Casting|CastToBP_Candle OtherActor)) ; Overlap candle actor?
  (if (Variables|Default|GetLightCandles)
    (Default|CandleLit _asbp_candle _returnvalue) ; On
    (else
      (Default|BlownOut _asbp_candle _returnvalue) ; Off
    )))

(fn ConstructionScript
  ;[1 1 1] Sets the... wait for it... the sphere radius!
  (Components|Sphere|SetSphereRadius (Variables|Default|GetSphere) (Variables|Default|GetSphereRadius) false))