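; Growable organic actor that scales its mesh up from near zero via a timeline after a delay, or starts full-size when growth is skipped.
; It plays growth audio, then a finale sound, notifies its Kernel on maturity, and destroys the Kernel when itself destroyed.
; It updates per-HealthDataType counts on the player's BP_LandscapeVisualModification component.
; A sphere, sized by GrowableRadius or mesh bounds, shows only while the debugger command is active.
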(event Custom|Grow
  (bind _kernel (Variables|Default|GetKernel))
  (bind _asbp_my_maru_character (Utilities|Casting|CastToBP_MyMaruCharacter (Game|Player|GetPlayerPawn 0)))
  (Default|OnGrowingKernelProcess _asbp_my_maru_character self)
  (CallFunction|AddGrowingNumber false)
  (Components|Timeline|SetPlayRate (Variables|Default|GetGrowth) (/ 1.0 (Variables|Default|GetGrowthTime)))
  (Audio|Components|Audio|SetSound (Variables|Default|GetAudio) (Variables|Default|GetGrowSound))
  (if (Variables|Default|GetPlayGrowSound)
    (Variables|Default|SetPlayGrowSound false)
    (Audio|Components|Audio|Play (Variables|Default|GetAudio) 0.0)
    (bind _scale (Timeline|Growth Play)
      (:Update
        (Transformation|SetWorldScale3D (Variables|Character|GetMesh) (Math|Vector|MakeVector (Math|Float|Lerp 0.01 (Variables|Default|GetFinalScale) _scale) (Math|Float|Lerp 0.01 (Variables|Default|GetFinalScale) _scale) (Math|Float|Lerp 0.01 (Variables|Default|GetFinalScale) _scale))))
      (:Finished
        (Audio|Components|Audio|Stop (Variables|Default|GetAudio))
        (Audio|SpawnSoundatLocation (Variables|Default|GetGrowFinale) "0, 0, 0" "0, 0, 0" 0.2 1.0 0.0 0 0)
        (if (Utilities|DoesObjectImplementInterface _kernel "/Script/iostest.INotifyMature")
          (Class|INotifyMature|NotifyMature(Message) _kernel))))
    (else
      (Timeline|Growth Play))))

(event EventBeginPlay
  (bind _finalscale (Variables|Default|GetFinalScale))
  (Utilities|FlowControl|Sequence
    (:then_0
      (if (Variables|Default|GetbSkipGrowth)
        (Transformation|SetRelativeScale3D (Variables|Character|GetMesh) (Math|Vector|MakeVector _finalscale _finalscale _finalscale))
        (CallFunction|AddGrowingNumber true)
        (else
          (Transformation|SetRelativeScale3D (Variables|Character|GetMesh) "0.010000,0.010000,0.010000")
          (bind _asbp_my_maru_character (Utilities|Casting|CastToBP_MyMaruCharacter (Game|Player|GetPlayerPawn 0)))
          (Math|Integer|IncrementInt (Variables|/Game/Blueprints/BP_MyMaruCharacter.BP_MyMaruCharacter_C|GetGrowingCounter _asbp_my_maru_character)
            (:%20%20
              (Utilities|FlowControl|Delay (Variables|Default|GetDelayScale))
              (CallFunction|Grow))))))
    (:then_1
      (CallFunction|SetSphereRadius))))

(event EventDestroyed
  (bind _kernel (Variables|Default|GetKernel))
  (CallFunction|RemoveGrowingNumber)
  (Utilities|IsValid _kernel
    (:Is%20Valid
      (Actor|DestroyActor _kernel))))

(event EventTick
  (params (DeltaSeconds :type Float%20%28single-precision%29))
  (Development|SetHiddeninGame (Variables|Default|GetSphere) (not (Class|HelperBlueprintFunction|IsDebuggerCommandActive)) false))

(fn ConstructionScript)

(fn AddGrowingNumber
  (params (SkipGrowingProcess :type Boolean))
  (bind _returnvalue (Game|Player|GetPlayerPawn 0))
  (bind _healthdatatype (Variables|Default|GetHealthDataType))
  (bind _returnvalue_2 (Actor|GetComponentbyClass _returnvalue "/Game/Blueprints/ActorComponent/BP_LandscapeVisualModification.BP_LandscapeVisualModification_C"))
  (bind _numberofgrowables (Variables|/Game/Blueprints/ActorComponent/BP_LandscapeVisualModification.BP_LandscapeVisualModification_C|GetNumberOfGrowables _returnvalue_2))
  (bind (_value _returnvalue_3) (Utilities|Map|Find _numberofgrowables _healthdatatype))
  (Utilities|IsValid _returnvalue
    (:Is%20Valid
      (Utilities|IsValid _returnvalue_2
        (:Is%20Valid
          (Utilities|FlowControl|Sequence
            (:then_0
              (if _returnvalue_3
                (Utilities|Map|Add _numberofgrowables (Variables|Default|GetHealthDataType) (+ _value 1))
                (else
                  (Utilities|Map|Add _numberofgrowables (Variables|Default|GetHealthDataType) 1))))
            (:then_1
              (Default|CallOnGrowableAdded _returnvalue_2 SkipGrowingProcess (/ 1.0 (Variables|Default|GetGrowthTime)) (Variables|Default|GetHealthDataType)))))))))

(fn RemoveGrowingNumber
  (bind _returnvalue (Game|Player|GetPlayerPawn 0))
  (bind _healthdatatype (Variables|Default|GetHealthDataType))
  (bind _returnvalue_2 (Actor|GetComponentbyClass _returnvalue "/Game/Blueprints/ActorComponent/BP_LandscapeVisualModification.BP_LandscapeVisualModification_C"))
  (bind _numberofgrowables (Variables|/Game/Blueprints/ActorComponent/BP_LandscapeVisualModification.BP_LandscapeVisualModification_C|GetNumberOfGrowables _returnvalue_2))
  (bind (_value _returnvalue_3) (Utilities|Map|Find _numberofgrowables _healthdatatype))
  (Utilities|IsValid _returnvalue
    (:Is%20Valid
      (Utilities|IsValid _returnvalue_2
        (:Is%20Valid
          (Utilities|FlowControl|Sequence
            (:then_0
              (if _returnvalue_3
                (Utilities|Map|Add _numberofgrowables (Variables|Default|GetHealthDataType) (+ _value -1))
                (else
                  (Utilities|Map|Add _numberofgrowables (Variables|Default|GetHealthDataType) 0))))
            (:then_1
              (Default|CallOnGrowableRemoved _returnvalue_2 (Variables|Default|GetHealthDataType)))))))))

(fn SetSphereRadius
  (bind _growableradius (Variables|Default|GetGrowableRadius))
  (Components|Sphere|SetSphereRadius (Variables|Default|GetSphere) (Math|Float|SelectFloat (.SphereRadius (Collision|GetComponentBounds (Variables|Character|GetMesh))) _growableradius (Math|Float|NearlyEqual(Float) _growableradius 0.0 1e-06)) true))