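; BP_Kernel is a kernel actor color-coded by activity type: move calories, exercise minutes, stand hours or social engagement.
; On BeginPlay it applies that color to a dynamic mesh material and point light, and sizes its sphere to the growable radius.
; Tick shows the sphere only while a debugger command is active.
; A brightness pulse timeline is present but never runs.
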(event EventBeginPlay
  (Utilities|FlowControl|Sequence
    (:then_0
      (Utilities|String|LogString "BEGIN Kernel")
      (bind _returnvalue (Rendering|Material|CreateDynamicMaterialInstance (Variables|Default|GetStaticMesh) 0 0 "None" :!class /Script/Engine.PrimitiveComponent))
      (Variables|Default|SetDIM_Kernal _returnvalue)
      (bind _color (CallFunction|GetColor (Variables|Default|GetType)))
      (Rendering|Material|SetVectorParameterValue (Variables|Default|GetDIM_Kernal) "Color" (Math|Conversions|ToLinearColor(Color) _color) :!class /Script/Engine.MaterialInstanceDynamic)
      (Rendering|Components|Light|SetLightColor (Variables|Default|GetPointLight) (Math|Conversions|ToLinearColor(Color) _color) true)
      (Utilities|String|LogString "END Kernel"))
    (:then_1
      (Components|Sphere|SetSphereRadius (Variables|Default|GetSphere) (Class|Kernel|GetGrowableRadius) true))))

(event EventTick
  (params (DeltaSeconds :type Float%20%28single-precision%29))
  (Development|SetHiddeninGame (Variables|Default|GetSphere) (not (Class|HelperBlueprintFunction|IsDebuggerCommandActive)) false))

(fn ConstructionScript)

(fn GetColor
  (params (Type :type EHealthDataType%20Enum :default "MoveCalories"))
  (switch Utilities|FlowControl|Switch|SwitchonEHealthDataType Type
    (:MoveCalories
      (return (Variables|Default|GetRed)))
    (:ExerciseMinutes
      (return (Variables|Default|GetGreen)))
    (:StandHoursCount
      (return (Variables|Default|GetBlue)))
    (:SocialEngagement
      (return (Variables|Default|GetYellow)))))