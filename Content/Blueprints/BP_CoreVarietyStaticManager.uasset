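; BP_CoreVarietyStaticManager is meant to vary the sand-to-grass blend across a list of landscapes, but its logic is currently disconnected.
; The unwired construction script code gives landscapes dynamic instances of MI_Landscape, using a "MID" name-prefix check, and sets SandToGrass from a parallel value array.
; The unwired event graph code reapplies those values to existing dynamic materials.
; Both the Update event and construction script are empty as wired.
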(event Custom|Update)

(fn ConstructionScript)